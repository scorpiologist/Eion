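; Player controller for mouse-driven voxel world editing, using sphere, box and projection tools configured through a UI widget.
; Tick finds the voxel world and hit under the cursor, reads Ctrl as Add, and updates spawned preview markers.
; Clicks apply sphere or box edits, while a looping timer repeats projection edits during a hold; each edit turns floating blocks into physics-simulated parts.
; Mouse wheel adjusts radius and H toggles the UI.
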(event Custom|ProjectionEditEvent
  (bind _ui (Variables|Default|GetUI))
  ;[1 1 1] Projection edit
  (bind _tool (Default|GetSelectedTool (Variables|Default|GetUI)))
  (if (and (>= (Class|PlayerController|GetInputKeyTimeDown "LeftMouseButton") (Variables|Parameters|GetEditDelay)) (Utilities|Enum|Equal(Enum) _tool "NewEnumerator0"))
    (bind _mode (Default|GetSelectedMode _ui))
    (bind (_strength _radius _materialindex _layer _debug) (Default|GetOptions _ui))
    (CallFunction|VoxelEdit (Variables|CurrentVariables|GetCurrentVoxelWorld) (Variables|CurrentVariables|GetCurrentHitPosition) (Variables|CurrentVariables|GetCurrentHitNormal) "NewEnumerator0" _mode (Variables|CurrentVariables|GetAdd) _strength _radius _materialindex _layer _debug (Variables|Parameters|GetProjectionToolHeight))
    (Class|VoxelTools|RemoveFloatingBlocks (Variables|CurrentVariables|GetCurrentVoxelWorld) "/Script/Voxel.VoxelPartSimpleMesh" (Variables|CurrentVariables|GetCurrentHitPosition) 5.0)
    (Class|VoxelTools|SimulatePhysicsonFloatingVoxelActors (Variables|CurrentVariables|GetCurrentVoxelWorld) (Variables|CurrentVariables|GetCurrentHitPosition) 10)))

(event EventBeginPlay
  ;[1 1 1] Init
  (Variables|Default|SetbShowMouseCursor true)
  (Utilities|Time|SetTimerbyEvent (delegate Custom|ProjectionEditEvent) (Variables|Parameters|GetEditDelay) true)
  (bind _returnvalue (UserInterface|CreateWidget (Variables|Parameters|GetUI%20Class) self))
  (bind _output_get (Variables|Default|SetUI _returnvalue))
  (UserInterface|Viewport|AddtoViewport _output_get 0)
  (CallFunction|SpawnMarkers))

(event EventTick
  (params (DeltaSeconds :type Float%20%28single-precision%29))
  (bind _ui (Variables|Default|GetUI))
  ;[1 1 1] Tick
  (if (Pawn|IsLocalPlayerController)
    (CallFunction|SetCurrentVariables)
    (bind _radius (Default|GetOptions _ui))
    (bind _tool (Default|GetSelectedTool _ui))
    (bind _mode (Default|GetSelectedMode _ui))
    (CallFunction|SetVoxelMarker (Variables|Markers|GetSphere) (Variables|Markers|GetSpotlight) (Variables|Markers|GetBox) (Variables|CurrentVariables|GetCurrentVoxelWorld) _tool _mode (Variables|CurrentVariables|GetCurrentHitPosition) (Variables|CurrentVariables|GetCurrentHitNormal) (Variables|Parameters|GetSpotlightHeight) (Variables|Parameters|GetProjectionToolHeight) _radius (Variables|CurrentVariables|GetAdd))))

(event Input|MouseEvents|MouseWheelAxis
  (params (AxisValue :type Float%20%28single-precision%29))
  ;[1 1 1] Radius
  (Default|IncreaseRadius (Variables|Default|GetUI) (* AxisValue (Variables|Parameters|GetRadiusChangeSpeed))))

(event Input|KeyboardEvents|H
  (params (Key :type Key%20Structure))
  (bind _ui (Variables|Default|GetUI))
  ;[1 1 1] Hide UI
  (:Pressed
    (switch Utilities|FlowControl|Switch|SwitchonESlateVisibility (Widget|GetVisibility _ui)
      (:Visible
        (Widget|SetVisibility _ui "Hidden" :!label _label))
      (:Hidden
        (Widget|SetVisibility _ui "Visible"))
      (:SelfHitTestInvisible
        (goto _label)))))

(event Input|MouseEvents|LeftMouseButton
  (params (Key :type Key%20Structure))
  (bind _ui (Variables|Default|GetUI))
  ;[1 1 1] Sphere/Box edit
  (:Pressed
    (bind _mode (Default|GetSelectedMode _ui))
    (bind _tool (Default|GetSelectedTool _ui))
    (bind (_strength _radius _materialindex _layer _debug) (Default|GetOptions _ui))
    (switch Utilities|FlowControl|Switch|SwitchonEVoxelTool _tool
      (:NewEnumerator1
        _)
      (:NewEnumerator2
        _))
    (CallFunction|VoxelEdit (Variables|CurrentVariables|GetCurrentVoxelWorld) (Variables|CurrentVariables|GetCurrentHitPosition) (Variables|CurrentVariables|GetCurrentHitNormal) _tool _mode (Variables|CurrentVariables|GetAdd) _strength _radius _materialindex _layer _debug 0.0)
    (Class|VoxelTools|RemoveFloatingBlocks (Variables|CurrentVariables|GetCurrentVoxelWorld) "/Script/Voxel.VoxelPartSimpleMesh" (Variables|CurrentVariables|GetCurrentHitPosition) 5.0)
    (Class|VoxelTools|SimulatePhysicsonFloatingVoxelActors (Variables|CurrentVariables|GetCurrentVoxelWorld) (Variables|CurrentVariables|GetCurrentHitPosition) 10)))

(fn ConstructionScript)

(fn SetCurrentVariables
  (bind _self self)
  (bind (_worldposition _worlddirection) (Class|VoxelTools|GetMouseWorldPositionandDirection _self)
    (:Success
      (bind (_world _hitposition _hitnormal) (Class|VoxelTools|GetVoxelWorld _worldposition _worlddirection (Variables|Parameters|GetMaxEditDistance) _self true))
      (Utilities|IsValid _world
        (:Is%20Valid
          (Variables|CurrentVariables|SetCurrentVoxelWorld _world))
        (:Is%20Not%20Valid
          _))
      (Variables|CurrentVariables|SetCurrentHitPosition _hitposition)
      (Variables|CurrentVariables|SetCurrentHitNormal _hitnormal)
      (Variables|CurrentVariables|SetAdd (or (>= (Class|PlayerController|GetInputKeyTimeDown "LeftControl") (Variables|Parameters|GetEditDelay)) (>= (Class|PlayerController|GetInputKeyTimeDown "RightControl") (Variables|Parameters|GetEditDelay)))))))

(fn SpawnMarkers
  (bind _returnvalue (Game|SpawnActorfromClass "/Voxel/Markers/BP_VoxelSphereMarker.BP_VoxelSphereMarker_C" (Math|Transform|MakeTransform "0, 0, 0") "Undefined" 0 (Game|Player|GetPlayerPawn 0)))
  (Variables|Markers|SetSphere _returnvalue)
  (bind _returnvalue_2 (Game|SpawnActorfromClass "/Voxel/Markers/BP_VoxelSpotLightMarker.BP_VoxelSpotLightMarker_C" (Math|Transform|MakeTransform "0, 0, 0") "Undefined" 0 (Game|Player|GetPlayerPawn 0)))
  (Variables|Markers|SetSpotlight _returnvalue_2)
  (bind _returnvalue_3 (Game|SpawnActorfromClass "/Voxel/Markers/BP_VoxelBoxMarker.BP_VoxelBoxMarker_C" (Math|Transform|MakeTransform "0, 0, 0") "Undefined" 0 (Game|Player|GetPlayerPawn 0)))
  (Variables|Markers|SetBox _returnvalue_3))