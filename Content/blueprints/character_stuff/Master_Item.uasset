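; Master_Item is a pickup item base that shows a prompt widget while the player character is within its trigger.
; The construction script fills the ItemInfo inventory struct from its image, text, action and self-reference, and applies the custom mesh.
; BeginPlay creates the PickUpWidget with that text, and trigger overlaps add or remove it and toggle IsInRange.
; The pickup action itself is not handled here.
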(event OnComponentBeginOverlap(trigger)
  (params (OverlappedComponent :type Primitive%20Component%20Object%20Reference) (OtherActor :type Actor%20Object%20Reference) (OtherComp :type Primitive%20Component%20Object%20Reference) (OtherBodyIndex :type Integer) (bFromSweep :type Boolean) (SweepResult :type Hit%20Result%20Structure%20%28by%20ref%29))
  (Utilities|Casting|CastToMYCHARACTER OtherActor)
  (UserInterface|Viewport|AddtoViewport (Variables|Default|GetpickUpWidget) 0)
  (Variables|Default|SetIsInRange true))

(event OnComponentEndOverlap(trigger)
  (params (OverlappedComponent :type Primitive%20Component%20Object%20Reference) (OtherActor :type Actor%20Object%20Reference) (OtherComp :type Primitive%20Component%20Object%20Reference) (OtherBodyIndex :type Integer))
  (Utilities|Casting|CastToMYCHARACTER OtherActor)
  (Widget|RemovefromParent (Variables|Default|GetpickUpWidget))
  (Variables|Default|SetIsInRange false))

(event EventBeginPlay
  (bind _iteminfo (Variables|Default|GetItemInfo))
  (bind _returnvalue (UserInterface|CreateWidget "/Game/blueprints/character_stuff/PickUpWidget.PickUpWidget_C"))
  (Variables|Default|SetpickUpWidget _returnvalue)
  (Variables|/Game/blueprints/character_stuff/PickUpWidget.PickUpWidget_C|SetPickUpActor _returnvalue 0)
  (Variables|/Game/blueprints/character_stuff/PickUpWidget.PickUpWidget_C|SetPickUpText _returnvalue (.PickUpText (Utilities|Struct|BreakInentory_structure _iteminfo)))
  (Utilities|Struct|SetmembersinInentory_structure _iteminfo self))

(fn ConstructionScript
  (Utilities|Struct|SetmembersinInentory_structure (Variables|Default|GetItemInfo) self (Variables|Default|GetItemImage) (Variables|Default|GetpickUpText) (Variables|Default|GetActionText))
  (Components|StaticMesh|SetStaticMesh (Variables|Default|GetStaticMesh) (Variables|Default|GetCustomMesh)))